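; Pursuit spline actor that draws a mesh visualisation of an AI pursuit path.
; Construction calls UpdateVisualisation, which syncs point data and, if enabled, rebuilds one non-colliding, shadowless spline mesh per segment.
; Each mesh follows point locations and tangents, with width from per-point data and roll adjusted by ConvertRoll to handle differences over 180 degrees.
; Helpers for point text labels and yaw flipping are defined but not called here.
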(event EventUpdateVisualisation
  (Class|PursuitSplineActor|SynchronisePointData)
  (if (Variables|Default|GetVisualisationEnabled)
    (Variables|Default|SetNumPoints (- (Spline|GetNumberOfSplinePoints (Variables|Default|GetPursuitSpline)) 1))
    (Variables|Default|SetNumSegments (- (Class|PursuitSplineComponent|GetNumberOfSplineSegments (Variables|Default|GetPursuitSpline)) 1))
    (CallFunction|GenerateSplineVisualisation)))

(fn ConstructionScript
  (Class|PursuitSplineActor|UpdateVisualisation))

(fn GenerateSplineVisualisation
  (for _array_element (Actor|GetComponentsByClass "/Script/Engine.SplineMeshComponent")
    (Components|DestroyComponent _array_element)
    (Transformation|DetachFromComponent _array_element "KeepRelative" "KeepRelative" "KeepRelative" true))
  (Class|PursuitSplineComponent|EmptySplineMeshes (Variables|Default|GetPursuitSpline))
  (for _index (range 0 (Variables|Default|GetNumSegments))
    (bind _returnvalue (AddComponent|AddPursuitSplineMeshComponent false))
    (Components|StaticMesh|SetStaticMesh _returnvalue "/Game/AI/S_PursuitSpline.S_PursuitSpline")
    (Class|PursuitSplineMeshComponent|SetupSplineComponent _returnvalue (Variables|Default|GetPursuitSpline) _index (Class|PursuitSplineComponent|ClampedNextIndex (Variables|Default|GetPursuitSpline) _index) (Variables|Default|GetSelected))
    (Utilities|FlowControl|Sequence
      (:then_0
        (SplineMesh|SetStartandEnd _returnvalue (.Location (Spline|GetLocationandTangentatSplinePoint (Variables|Default|GetPursuitSpline) _index "Local")) (.Tangent (Spline|GetLocationandTangentatSplinePoint (Variables|Default|GetPursuitSpline) _index "Local")) (.Location (Spline|GetLocationandTangentatSplinePoint (Variables|Default|GetPursuitSpline) (Class|PursuitSplineComponent|ClampedNextIndex (Variables|Default|GetPursuitSpline) _index) "Local")) (.Tangent (Spline|GetLocationandTangentatSplinePoint (Variables|Default|GetPursuitSpline) (Class|PursuitSplineComponent|ClampedNextIndex (Variables|Default|GetPursuitSpline) _index) "Local")) true :!class /Script/Engine.SplineMeshComponent))
      (:then_1
        (SplineMesh|SetStartScale _returnvalue (Math|Vector2D|MakeVector2D (Class|PursuitSplineComponent|GetWidthatSplinePoint (Variables|Default|GetPursuitSpline) _index) 0.0) true :!class /Script/Engine.SplineMeshComponent))
      (:then_2
        (SplineMesh|SetEndScale _returnvalue (Math|Vector2D|MakeVector2D (Class|PursuitSplineComponent|GetWidthatSplinePoint (Variables|Default|GetPursuitSpline) (Class|PursuitSplineComponent|ClampedNextIndex (Variables|Default|GetPursuitSpline) _index)) 0.0) true :!class /Script/Engine.SplineMeshComponent))
      (:then_3
        (Collision|SetCollisionEnabled _returnvalue "NoCollision"))
      (:then_4
        (Class|SplineMeshComponent|SetStartRoll _returnvalue (.OutputRoll1 (CallFunction|ConvertRoll (Spline|GetRollatSplinePoint (Variables|Default|GetPursuitSpline) _index "Local") (Spline|GetRollatSplinePoint (Variables|Default|GetPursuitSpline) (Class|PursuitSplineComponent|ClampedNextIndex (Variables|Default|GetPursuitSpline) _index) "Local"))) true))
      (:then_5
        (Class|SplineMeshComponent|SetEndRoll _returnvalue (.OutputRoll2 (CallFunction|ConvertRoll (Spline|GetRollatSplinePoint (Variables|Default|GetPursuitSpline) _index "Local") (Spline|GetRollatSplinePoint (Variables|Default|GetPursuitSpline) (Class|PursuitSplineComponent|ClampedNextIndex (Variables|Default|GetPursuitSpline) _index) "Local"))) true))
      (:then_6
        (Rendering|SetCastShadow _returnvalue false)))))

(fn SetupPointText
  (params (TextComponent :type Text%20Render%20Component%20Object%20Reference) (Text :type Text) (WorldSize :type Float%20%28single-precision%29) (Colour :type Linear%20Color%20Structure) (Location :type Vector) (Rotation :type Rotator))
  (Utilities|FlowControl|Sequence
    (:then_0
      (Transformation|SetRelativeLocationAndRotation TextComponent Location Rotation false false))
    (:then_1
      (Rendering|Components|TextRender|SetText TextComponent Text))
    (:then_2
      (Rendering|Components|TextRender|SetWorldSize TextComponent WorldSize))
    (:then_3
      (Rendering|Components|TextRender|SetHorizontalAlignment TextComponent "EHTA_Center"))
    (:then_4
      (Rendering|Components|TextRender|SetTextRenderColor TextComponent (Math|Conversions|ToColor(LinearColor) Colour)))))

(fn RotateYaw180
  (params (Rotation :type Rotator))
  (bind (_roll _pitch _yaw) (Math|Rotator|BreakRotator Rotation))
  (return (Math|Rotator|MakeRotator (* _roll -1.0) _pitch (+ _yaw 1.8e+02))))

(fn ConvertRoll
  (params (InputRoll1 :type Float%20%28single-precision%29) (InputRoll2 :type Float%20%28single-precision%29))
  (Math|Float|CompareFloat (Math|Float|Absolute(Float) (- InputRoll1 InputRoll2)) 1.8e+02
    (:>
      (return (Math|Trig|DegreesToRadians (CallFunction|ConstrainAngle InputRoll1)) (Math|Trig|DegreesToRadians (CallFunction|ConstrainAngle InputRoll2))))
    (:==
      _)
    (:<
      _))
  (return (Math|Trig|DegreesToRadians InputRoll1) (Math|Trig|DegreesToRadians InputRoll2)))

(fn ConstrainAngle
  (params (Input :type Float%20%28single-precision%29))
  (Math|Float|CompareFloat Input 0.0
    (:>
      _)
    (:==
      _)
    (:<
      (return (+ 3.6e+02 Input))))
  (return Input))
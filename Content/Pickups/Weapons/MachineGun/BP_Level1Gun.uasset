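; Level 1 machine gun Blueprint that plays particle and sound effects when its rounds hit something.
; BulletHitAnimation attaches any supplied particle systems to the hit component, with a shield-hit sound as fallback.
; Otherwise it switches on surface type to spawn impact effects, tinting dirt, sand, snow and rock by the passed colour.
; Vehicle hits attach to the component and use a harder effect when charged.
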(event EventBulletHitAnimation
  (params (component :type Primitive%20Component%20Object%20Reference) (particleSystems :type Array%20of%20Particle%20System%20Object%20References) (hitLocations :type Array%20of%20Vectors) (soundEffect :type Sound%20Cue%20Object%20Reference) (location :type Vector%20%28by%20ref%29 :default "0, 0, 0") (rotation :type Rotator%20%28by%20ref%29 :default "0, 0, 0") (surface :type EGameSurface%20Enum :default "Default") (colour :type Vector%20%28by%20ref%29 :default "0, 0, 0") (charged :type Boolean))
  ;[1 1 1] Round impact with surfaces
  (Math|Integer|CompareInt (Utilities|Array|Length particleSystems)
    (:>
      (for (_array_element _array_index) particleSystems
        (bind _returnvalue (Effects|SpawnEmitterAttached _array_element component "RootDummy" (Utilities|Array|Get(acopy) hitLocations _array_index)))
        (Transformation|SetRelativeScale3D _returnvalue "1.000000,1.000000,1.000000"))
      (if (Utilities|IsValid soundEffect)
        (Audio|SpawnSoundAttached soundEffect component "None" "0, 0, 0" "0, 0, 0" "KeepRelativeOffset" true 1.0 1.0 0.0 0 0)
        (else
          (Audio|SpawnSoundAttached "/Game/Audio/Sounds/Pickups/Shield/A_ShieldHit_Cue.A_ShieldHit_Cue" component "None" "0, 0, 0" "0, 0, 0" "KeepRelativeOffset" true 1.0 1.0 0.0 0 0))))
    (:==
      (switch Utilities|FlowControl|Switch|SwitchonEGameSurface surface :!label _label
        (:Asphalt
          (Effects|SpawnEmitteratLocation "/Game/Pickups/Weapons/MachineGun/HitEffects/PS_HitConcrete.PS_HitConcrete" location rotation :!label _label_2)
          (Audio|SpawnSoundatLocation "/Game/Audio/Sounds/Pickups/Weapons/MachineGun/A_HitRock_Cue.A_HitRock_Cue" location "0, 0, 0" 1.0 1.0 0.0 0 0))
        (:Dirt
          (bind _returnvalue_2 (Effects|SpawnEmitteratLocation "/Game/Pickups/Weapons/MachineGun/HitEffects/PS_HitSand.PS_HitSand" location rotation :!label _label_3))
          (Effects|Components|ParticleSystem|SetVectorParameter _returnvalue_2 "SurfaceColour" colour)
          (Audio|SpawnSoundatLocation "/Game/Audio/Sounds/Pickups/Weapons/MachineGun/MG_John/A_Imp_CG_Sand01_Cue.A_Imp_CG_Sand01_Cue" location "0, 0, 0" 1.0 1.0 0.0 0 0))
        (:Wood
          (Effects|SpawnEmitteratLocation "/Game/Pickups/Weapons/MachineGun/HitEffects/PS_HitWood.PS_HitWood" location rotation)
          (Audio|SpawnSoundatLocation "/Game/Audio/Sounds/Pickups/Weapons/MachineGun/A_HitRock_Cue.A_HitRock_Cue" location "0, 0, 0" 1.0 1.0 0.0 0 0))
        (:Rock
          (bind _returnvalue_3 (Effects|SpawnEmitteratLocation "/Game/Pickups/Weapons/MachineGun/HitEffects/PS_HitRock.PS_HitRock" location rotation))
          (Effects|Components|ParticleSystem|SetVectorParameter _returnvalue_3 "SurfaceColour" colour)
          (Audio|SpawnSoundatLocation "/Game/Audio/Sounds/Pickups/Weapons/MachineGun/A_HitRock_Cue.A_HitRock_Cue" location "0, 0, 0" 1.0 1.0 0.0 0 0))
        (:Metal
          (Effects|SpawnEmitteratLocation "/Game/Pickups/Weapons/MachineGun/HitEffects/PS_HitMetal.PS_HitMetal" location rotation)
          (Audio|SpawnSoundatLocation "/Game/Audio/Sounds/Pickups/Weapons/MachineGun/A_MGHitMetal_Cue.A_MGHitMetal_Cue" location "0, 0, 0" 1.0 1.0 0.0 0 0))
        (:Gravel
          (goto _label_2))
        (:Sand
          (goto _label_3))
        (:Field
          (Effects|SpawnEmitteratLocation "/Game/Maps/Track1/Environment/RaceTrack/RaceBarrier/PS_RaceBarrierMGHit.PS_RaceBarrierMGHit" location rotation)
          (Audio|SpawnSoundatLocation "/Game/Audio/Sounds/Impacts/A_ForceFieldImpact_Cue.A_ForceFieldImpact_Cue" location "0, 0, 0" 1.0 1.0 0.0 0 0))
        (:Vehicle
          (if charged
            (Effects|SpawnEmitterAttached "/Game/Pickups/Weapons/MachineGun/HitEffects/PS_HitVehicleHard.PS_HitVehicleHard" component "RootDummy" location rotation "1.000000,1.000000,1.000000" "KeepWorldPosition")
            (else
              (Effects|SpawnEmitterAttached "/Game/Pickups/Weapons/MachineGun/HitEffects/PS_HitVehicle.PS_HitVehicle" component "RootDummy" location rotation "1.000000,1.000000,1.000000" "KeepWorldPosition")))
          (Audio|SpawnSoundAttached "/Game/Audio/Sounds/Pickups/Weapons/MachineGun/A_MGHitMetal_Cue.A_MGHitMetal_Cue" component "None" "0, 0, 0" "0, 0, 0" "KeepRelativeOffset" true 1.0 1.0 0.0 0 0))
        (:Snow
          (goto _label_3))))
    (:<
      (goto _label))))

(fn ConstructionScript)
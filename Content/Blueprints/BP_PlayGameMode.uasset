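; BP_PlayGameMode is the game mode for play, covering player spawning, audio volume and XP pickup messages.
; SetAudioOptionsforVolume reads the audio options from the GlobalGameState game instance and sets effects, UI and music sound class volumes, zeroing muted groups.
; It overrides player start selection via ChoosePlayerStartProperly because default selection fails, and returns the default pawn class.
; GetXPMessage formats XP text with a header chosen by pickup type.
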(event EventSetAudioOptionsforVolume
  (bind _asglobal_game_state (Utilities|Casting|CastToGlobalGameState (Game|GetGameInstance)))
  (Utilities|FlowControl|Sequence
    (:then_0
      (if (.MuteEffects (Utilities|Struct|BreakAudioOptions (Variables|/Script/Grip.GlobalGameState|GetAudioOptions _asglobal_game_state)))
        (Class|GlobalGameState|SetSoundClassVolume "/Game/Audio/SoundClasses/SFX.SFX" 0.0)
        (Class|GlobalGameState|SetSoundClassVolume "/Game/Audio/SoundClasses/UI.UI" 0.0)
        (Class|GlobalGameState|SetSoundClassVolume "/Game/Audio/SoundClasses/OutOfBand_SFX.OutOfBand_SFX" 0.0)
        (else
          (Class|GlobalGameState|SetSoundClassVolume "/Game/Audio/SoundClasses/SFX.SFX" (.EffectsVolumeLevel (Utilities|Struct|BreakAudioOptions (Variables|/Script/Grip.GlobalGameState|GetAudioOptions _asglobal_game_state))))
          (Class|GlobalGameState|SetSoundClassVolume "/Game/Audio/SoundClasses/UI.UI" (.EffectsVolumeLevel (Utilities|Struct|BreakAudioOptions (Variables|/Script/Grip.GlobalGameState|GetAudioOptions _asglobal_game_state))))
          (Class|GlobalGameState|SetSoundClassVolume "/Game/Audio/SoundClasses/OutOfBand_SFX.OutOfBand_SFX" (.EffectsVolumeLevel (Utilities|Struct|BreakAudioOptions (Variables|/Script/Grip.GlobalGameState|GetAudioOptions _asglobal_game_state)))))))
    (:then_1
      (if (.MuteMusic (Utilities|Struct|BreakAudioOptions (Variables|/Script/Grip.GlobalGameState|GetAudioOptions _asglobal_game_state)))
        (Class|GlobalGameState|SetSoundClassVolume "/Game/Audio/SoundClasses/Music.Music" 0.0)
        (else
          (Class|GlobalGameState|SetSoundClassVolume "/Game/Audio/SoundClasses/Music.Music" (.MusicVolumeLevel (Utilities|Struct|BreakAudioOptions (Variables|/Script/Grip.GlobalGameState|GetAudioOptions _asglobal_game_state)))))))))

(fn ConstructionScript)

(fn ChoosePlayerStart
  (params (Player :type Controller%20Object%20Reference))
  ;[1 1 1] We have to override player start selection so that it actually works
  (bind _returnvalue (Class|PlayGameMode|ChoosePlayerStartProperly Player))
  (return _returnvalue))

(fn GetDefaultPawnClassforController
  (params (InController :type Controller%20Object%20Reference))
  (return (Variables|Default|GetDefaultPawnClass)))

(fn GetXPMessage
  (params (pickupType :type EPickupType%20Enum :default "None") (numPoints :type Integer))
  (return (Utilities|Text|FormatText "{XPType} +{XPAmount}" (UI|GetXPMessageHeader pickupType) (Utilities|Text|ToText(Integer) numPoints))))

(fn GetXPMessageHeader
  (params (pickupType :type EPickupType%20Enum :default "None"))
  (return (Utilities|Select :Index pickupType :None "" :Random "" :Shield "PAINKILLER DECIMATED" :TurboBoost "" :HomingMissile "SCORPION STING" :GatlingGun "RAPTOR RIPPING")))
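; Spline-driven racetrack forcefield barrier, built entirely in the Construction Script, with optional snapping of spline points to terrain via downward traces.
; When UncheckForManeuvering is on, spline meshes are laid at fixed spacing, with wall size, holo visibility and collision toggles.
; Scaled direction tangents smooth curves and spline roll banks the segments.
; Static junction posts follow at their own spacing, plus an end cap; point-light placement is disconnected.
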(event EventBeginPlay)

(event Collision|EventActorBeginOverlap
  (params (OtherActor :type Actor%20Object%20Reference)))

(event EventTick
  (params (DeltaSeconds :type Float%20%28single-precision%29)))

(fn ConstructionScript
  (bind _tangentscale (Variables|Default|GetTangentScale))
  (bind _spline (Variables|Default|GetSpline))
  (bind _spline_2 (Variables|Default|GetSpline))
  (bind _roll_sensitivity (Variables|Default|GetRoll%20Sensitivity))
  (bind _meshspacing (Variables|Default|GetMeshSpacing))
  (bind _spline_3 (Variables|Default|GetSpline))
  (bind _spline_4 (Variables|Default|GetSpline))
  (bind _spline_5 (Variables|Default|GetSpline))
  (bind _spacing (Variables|Default|GetSpacing))
  (bind _returnvalue (Spline|GetSplineLength _spline_2))
  (if (Variables|Default|GetSnap%20to%20Terrain?)
    (for _index (range 0 (Spline|GetNumberOfSplinePoints (Variables|Default|GetSpline)))
      (bind _outhit (Collision|LineTraceForObjects (Spline|GetLocationatSplinePoint _spline_4 _index "World") (+ (Spline|GetLocationatSplinePoint _spline_4 _index "World") "0, 0,-5000.000000") (Utilities|Array|MakeArray "ObjectTypeQuery1" "ObjectTypeQuery2") false 0 "None"))
      (Spline|SetLocationatSplinePoint _spline_4 _index (Math|Vector|MakeVector (.X (Math|Vector|BreakVector (Spline|GetLocationatSplinePoint _spline_4 _index "World"))) (.Y (Math|Vector|BreakVector (Spline|GetLocationatSplinePoint _spline_4 _index "World"))) (.Z (Math|Vector|BreakVector (.ImpactPoint (Collision|BreakHitResult _outhit))))) "World" true)))
  (for _index_2 (range 0 (.ReturnValue (Math|Float|Division(WholeandRemainder) _returnvalue _spacing)))
    (if (Variables|Default|GetUncheck%20for%20Maneuvering)
      (if (Variables|Default|GetBig%20wall?)
        ;[1 1 1] lrg
        (bind _returnvalue_2 (AddComponent|AddSplineMeshComponent true))
        (LocalVariables|SetSplineComponent _returnvalue_2)
        (else
          ;[1 1 1] sm
          (bind _returnvalue_3 (AddComponent|AddSplineMeshComponent true))
          (LocalVariables|SetSplineComponent _returnvalue_3)))
      (if (Variables|Default|GetHolo%20Visible?)
        (Rendering|SetVisibility (LocalVariables|GetSplineComponent) true false)
        (else
          (Rendering|SetVisibility (LocalVariables|GetSplineComponent) false false)))
      (if (Variables|Default|GetCollision)
        ;[1 1 1] Fence
        (Collision|SetCollisionEnabled (LocalVariables|GetSplineComponent) "QueryAndPhysics")
        (else
          (Collision|SetCollisionEnabled (LocalVariables|GetSplineComponent) "NoCollision")))
      (bind _returnvalue_4 (AddComponent|AddSplineMeshComponent true))
      (bind _returnvalue_5 (AddComponent|AddSplineMeshComponent true))
      (Collision|SetCollisionProfileName _returnvalue_5 "ForceField" true :!class /Script/Engine.PrimitiveComponent)
      (SplineMesh|SetStartandEnd _returnvalue_5 (Spline|GetLocationatDistanceAlongSpline _spline (* _index_2 _spacing) "World") (* (Spline|GetDirectionatDistanceAlongSpline _spline (* _index_2 _spacing) "World") _tangentscale) (Spline|GetLocationatDistanceAlongSpline _spline (+ (* _index_2 _spacing) _spacing) "World") (* (Spline|GetDirectionatDistanceAlongSpline _spline (+ (* _index_2 _spacing) _spacing) "World") _tangentscale) true :!class /Script/Engine.SplineMeshComponent)
      (Class|SplineMeshComponent|SetStartRoll _returnvalue_4 (* (Class|SplineComponent|GetRollatDistanceAlongSpline _spline_5 (* _index_2 _spacing) "World") _roll_sensitivity) true)
      (Class|SplineMeshComponent|SetEndRoll _returnvalue_4 (* (Class|SplineComponent|GetRollatDistanceAlongSpline _spline_5 (+ (* _index_2 _spacing) _spacing) "World") _roll_sensitivity) true)))
  (for _index_3 (range 0 (.ReturnValue (Math|Float|Division(WholeandRemainder) _returnvalue (Variables|Default|GetLightSpacing))))
    _)
  ;[1 1 1] Add Junctions at the correct spacings after placing lights
  (for _index_4 (range 0 (.ReturnValue (Math|Float|Division(WholeandRemainder) (Spline|GetSplineLength _spline_3) _meshspacing)))
    (AddComponent|AddStaticMeshComponent true (Math|Transform|MakeTransform (Spline|GetLocationatDistanceAlongSpline _spline_3 (* _index_4 _meshspacing) "World") (Spline|GetRotationatDistanceAlongSpline _spline_3 (* _index_4 _meshspacing) "World"))))
  (AddComponent|AddStaticMeshComponent true (Math|Transform|MakeTransform (Spline|GetLocationatSplinePoint (Variables|Default|GetSpline) (- (Spline|GetNumberOfSplinePoints (Variables|Default|GetSpline)) -1) "World") (Spline|GetRotationatDistanceAlongSpline _spline_3 (* _index_4 _meshspacing) "World"))))
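; Blueprint for the Artifex 1AG tank vehicle that drives its engine visual effects from inherited vehicle events.
; Thrust events toggle high exhaust effects, restart low exhaust when released, and change exhaust light intensity.
; Gear changes in either direction share a half-second backfire burst, while turbo events switch a turbo effect.
; A vehicle reset restores idle exhaust, clears the other effects and resets light intensity.
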(event EventGameResetVehicle
  ;[1 1 1] Reset the custom vehicle effects
  (Rendering|Components|Light|SetIntensity (Variables|Default|GetExhaustLightL2) 5e+02)
  (Components|Activation|Deactivate (Variables|Default|GetEngineBackfire))
  (Components|Activation|Activate (Variables|Default|GetEngineExhaustLow) true))

(event EventThrustEngaged
  ;[1 1 1] Thrust engaged
  (Utilities|FlowControl|Sequence
    (:then_0
      (Components|Activation|Activate (Variables|Default|GetEngineExhaustHigh) false))
    (:then_1
      (Rendering|Components|Light|SetIntensity (Variables|Default|GetExhaustLightL2) 7e+02))))

(event EventThrustDisengaged
  (bind _engineexhaustlow (Variables|Default|GetEngineExhaustLow))
  ;[1 1 1] Thrust disengaged
  (Utilities|FlowControl|Sequence
    (:then_0
      (Components|Activation|Deactivate _engineexhaustlow)
      (Components|Activation|Activate _engineexhaustlow false))
    (:then_1
      (Components|Activation|Deactivate (Variables|Default|GetEngineExhaustHigh)))
    (:then_2
      (Rendering|Components|Light|SetIntensity (Variables|Default|GetExhaustLightL2) 4e+02))))

(event EventGearUpEngaged
  (bind _enginebackfire (Variables|Default|GetEngineBackfire))
  ;[1 1 1] Gear change
  (Components|Activation|Activate _enginebackfire true)
  (Utilities|FlowControl|Delay 0.5)
  (Components|Activation|Deactivate _enginebackfire))

(event EventGearDownEngaged
  (bind _enginebackfire (Variables|Default|GetEngineBackfire))
  ;[1 1 1] Gear change
  (Components|Activation|Activate _enginebackfire true)
  (Utilities|FlowControl|Delay 0.5)
  (Components|Activation|Deactivate _enginebackfire))

(event EventTurboEngaged
  ;[1 1 1] Turbo activation
  (Components|Activation|Activate (Variables|Default|GetTurboEffect) false))

(event EventTurboDisengaged
  ;[1 1 1] Turbo activation
  (Components|Activation|Deactivate (Variables|Default|GetTurboEffect)))

(fn ConstructionScript
  (|CallParentFunction))
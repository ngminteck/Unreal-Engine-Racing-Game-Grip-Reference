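; DirectionSignBP is a planet signage actor that shows a direction through one of two light meshes.
; Its construction script applies the Material variable to both Lights and Lights2, then uses the Direction boolean to hide one of them.
; All setup happens at construction, and the event graph holds only disabled placeholder events.
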(event EventBeginPlay)

(event EventActorBeginOverlap
  (params (OtherActor :type Actor%20Object%20Reference)))

(event EventTick
  (params (DeltaSeconds :type Float%20%28single-precision%29)))

(fn ConstructionScript
  (bind _material (Variables|Default|GetMaterial))
  (Rendering|Material|SetMaterial (Variables|Default|GetLights) 0 _material)
  (Rendering|Material|SetMaterial (Variables|Default|GetLights2) 0 _material)
  (if (Variables|Default|GetDirection)
    (Rendering|SetVisibility (Variables|Default|GetLights2) false false)
    (else
      (Rendering|SetVisibility (Variables|Default|GetLights) false false))))
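; Construction-script spline tool that builds a tunnel or track from spline mesh segments along TrackSpline.
; It derives segment length from the road mesh bounds, stretches it to fit the spline, and resizes RoadDataArray to hold per-point bank, scale, orientation and mesh overrides.
; BuildTrackElement adds each segment, supporting first/last meshes, flipping, two additional mesh layers with switched collision, and roll-based banking.
; Optional text renders label track points.
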(event EventBeginPlay)

(event EventActorBeginOverlap
  (params (OtherActor :type Actor%20Object%20Reference)))

(event EventTick
  (params (DeltaSeconds :type Float%20%28single-precision%29)))

(fn ConstructionScript
  (bind _additionalmesh1 (Variables|TrackSetup|GetAdditionalMesh1))
  (bind _collision (Variables|TrackSetup|GetCollision))
  (bind _roadmesh (Variables|TrackSetup|GetRoadMesh))
  (bind _roaddataarray (Variables|TrackSetup|GetRoadDataArray))
  (bind _hideadditionalmesh1 (Variables|TrackSetup|GetHideAdditionalMesh1))
  (bind _additionalmesh1_2 (Variables|TrackSetup|GetAdditionalMesh1))
  (bind _additionalmesh2 (Variables|TrackSetup|GetAdditionalMesh2))
  (bind _trackspline (Variables|Default|GetTrackSpline))
  (bind _trackspline_2 (Variables|Default|GetTrackSpline))
  (bind _returnvalue (Utilities|IsValid _additionalmesh1))
  (bind _returnvalue_2 (Spline|GetSplineLength _trackspline_2))
  (bind _returnvalue_3 (StaticMesh|GetBoundingBox _roadmesh))
  (Utilities|FlowControl|Sequence
    (:then_0
      (if (and (Variables|TrackSetup|GetAutomaticSegmentLength) (Utilities|IsValid _roadmesh))
        (Variables|TrackSetup|SetSegmentLength (Utilities|Select :Index (Variables|TrackSetup|GetUniversalMeshOrientation) :X (- (.x (.max _returnvalue_3)) (.x (.min _returnvalue_3))) :Y (- (.y (.max _returnvalue_3)) (.y (.min _returnvalue_3))) :Z (- (.z (.max _returnvalue_3)) (.z (.min _returnvalue_3))))))
      (bind _output_get (LocalVariables|SetRoadMeshCollision (and _collision (not _returnvalue))))
      (LocalVariables|SetAlternateMesh2Collision _output_get)
      (LocalVariables|SetAlternateMesh1Collision (and _collision _returnvalue)))
    (:then_1
      (if (Variables|TrackSetup|GetLockSplineLength)
        _
        (else
          (bind _output_get_2 (Variables|TrackSetup|SetLockedSplineLength _returnvalue_2))))
      (bind _numpoints (CallFunction|GetNumPoints _output_get_2))
      (bind _output_get_3 (Variables|Default|SetPointsAmount _numpoints))
      (bind _numpoints_2 (CallFunction|GetNumPoints _returnvalue_2))
      (bind _output_get_4 (Variables|Default|SetLockedPointsAmount _numpoints_2))
      (Math|Float|CompareFloat (Math|Conversions|ToFloat(Integer) _output_get_3) 0.0
        (:>
          (Variables|TrackSetup|SetSegmentLength (* (Variables|TrackSetup|GetSegmentLength) (/ (Math|Conversions|ToFloat(Integer) _output_get_4) (Math|Conversions|ToFloat(Integer) _output_get_3))) :!label _label))
        (:==
          (Variables|TrackSetup|SetSegmentLength 0.0))
        (:<
          (goto _label))))
    (:then_2
      (if (Variables|TrackSetup|GetApplyMeshOrientation)
        (CallFunction|ApplyOrientation)
        (Variables|TrackSetup|SetApplyMeshOrientation false)
        (else
          (Utilities|Struct|SetmembersinRoadData (Variables|Default|GetRoadMeshDefaults) (Variables|TrackSetup|GetUniversalMeshOrientation))
          (Math|Integer|CompareInt (Utilities|Array|Length (Variables|TrackSetup|GetRoadDataArray)) (+ (Variables|Default|GetPointsAmount) 1) :!label _label_2
            (:>
              (Utilities|Array|RemoveIndex _roaddataarray (Utilities|Array|LastIndex _roaddataarray))
              (goto _label_2))
            (:<
              (Utilities|Array|Add (Variables|TrackSetup|GetRoadDataArray) (Utilities|Struct|MakeRoadData 1.0 1.0 (Variables|TrackSetup|GetUniversalMeshOrientation)))
              (goto _label_2))))))
    (:then_3
      (for _index (range 0 (- (Variables|Default|GetPointsAmount) 1))
        (Variables|Default|SetCurrentLoopIndex _index)
        (Utilities|FlowControl|Sequence
          (:then_0
            (if (Utilities|IsValid (.overridemesh (Utilities|Array|Get(acopy) (Variables|TrackSetup|GetRoadDataArray) (Variables|Default|GetCurrentLoopIndex))))
              (CallFunction|BuildTrackElement (Variables|Default|GetCurrentLoopIndex) (.overridemesh (Utilities|Array|Get(acopy) (Variables|TrackSetup|GetRoadDataArray) (Variables|Default|GetCurrentLoopIndex))) false (LocalVariables|GetRoadMeshCollision))
              (elif (and (Utilities|IsValid (Variables|FirstandLastMeshSettings|GetLastMesh)) (== (+ (Variables|Default|GetCurrentLoopIndex) 1) (Variables|Default|GetPointsAmount)))
                (CallFunction|BuildTrackElement (Variables|Default|GetCurrentLoopIndex) (Variables|FirstandLastMeshSettings|GetLastMesh) false (Variables|TrackSetup|GetCollision))
                (elif (and (Utilities|IsValid (Variables|FirstandLastMeshSettings|GetFirstMesh)) (== (Variables|Default|GetCurrentLoopIndex) 0))
                  (CallFunction|BuildTrackElement (Variables|Default|GetCurrentLoopIndex) (Variables|FirstandLastMeshSettings|GetFirstMesh) false (Variables|TrackSetup|GetCollision))
                  (else
                    (CallFunction|BuildTrackElement (Variables|Default|GetCurrentLoopIndex) (Variables|TrackSetup|GetRoadMesh) false (LocalVariables|GetRoadMeshCollision)))))))
          (:then_1
            (Utilities|IsValid (.collisionoverride (Utilities|Array|Get(acopy) (Variables|TrackSetup|GetRoadDataArray) (Variables|Default|GetCurrentLoopIndex)))
              (:Is%20Valid
                (CallFunction|BuildTrackElement (Variables|Default|GetCurrentLoopIndex) (.collisionoverride (Utilities|Array|Get(acopy) (Variables|TrackSetup|GetRoadDataArray) (Variables|Default|GetCurrentLoopIndex))) true (LocalVariables|GetAlternateMesh1Collision)))
              (:Is%20Not%20Valid
                (Utilities|IsValid _additionalmesh1_2
                  (:Is%20Valid
                    (CallFunction|BuildTrackElement (Variables|Default|GetCurrentLoopIndex) _additionalmesh1_2 true (LocalVariables|GetAlternateMesh1Collision)))))))
          (:then_2
            (Utilities|IsValid (.additionalmeshoverride (Utilities|Array|Get(acopy) (Variables|TrackSetup|GetRoadDataArray) (Variables|Default|GetCurrentLoopIndex)))
              (:Is%20Valid
                (CallFunction|BuildTrackElement (Variables|Default|GetCurrentLoopIndex) (.additionalmeshoverride (Utilities|Array|Get(acopy) (Variables|TrackSetup|GetRoadDataArray) (Variables|Default|GetCurrentLoopIndex))) _hideadditionalmesh1 (LocalVariables|GetAlternateMesh2Collision)))
              (:Is%20Not%20Valid
                (Utilities|IsValid _additionalmesh2
                  (:Is%20Valid
                    (CallFunction|BuildTrackElement (Variables|Default|GetCurrentLoopIndex) _additionalmesh2 _hideadditionalmesh1 (LocalVariables|GetAlternateMesh2Collision))))))))))
    (:then_4
      (if (Variables|TrackSetup|GetDrawTrackPoints)
        (for _index_2 (range 0 (Variables|Default|GetPointsAmount))
          (Variables|Default|SetCurrentTrackPoint (Utilities|Text|ToText(Integer) _index_2))
          (bind _returnvalue_4 (AddComponent|AddTextRenderComponent false (Math|Transform|MakeTransform (Math|Vector|MakeVector (.X (Math|Vector|BreakVector (Spline|GetLocationatDistanceAlongSpline _trackspline (* _index_2 (Variables|TrackSetup|GetSegmentLength)) "Local"))) (.Y (Math|Vector|BreakVector (Spline|GetLocationatDistanceAlongSpline _trackspline (* _index_2 (Variables|TrackSetup|GetSegmentLength)) "Local"))) (+ (+ (.Z (Math|Vector|BreakVector (Spline|GetLocationatDistanceAlongSpline _trackspline (* _index_2 (Variables|TrackSetup|GetSegmentLength)) "Local"))) 5e+02) (Variables|TrackSetup|GetTrackPointsHeight))) (Math|Conversions|RotationFromXVector (* (Spline|GetTangentatDistanceAlongSpline _trackspline (* _index_2 (Variables|TrackSetup|GetSegmentLength)) "Local") -1)))))
          (Rendering|Components|TextRender|SetText _returnvalue_4 (Variables|Default|GetCurrentTrackPoint)))))
    (:then_5
      (Variables|TrackSetup|SetFirst%20spline%20point%20location (Spline|GetLocationatSplinePoint (Variables|Default|GetTrackSpline) (Variables|TrackSetup|GetFirst%20spline%20point%20location%20#) "World"))
      (Variables|TrackSetup|SetLast%20spline%20point%20location (Spline|GetLocationatSplinePoint (Variables|Default|GetTrackSpline) (Variables|TrackSetup|GetLast%20spline%20point%20location%20#) "World")))))

(fn BuildTrackElement
  (params (LoopIndex :type Integer) (TrackElementMesh :type Static%20Mesh%20Object%20Reference) (HideInGame :type Boolean) (EnableCollision :type Boolean))
  (bind _trackspline (Variables|Default|GetTrackSpline))
  (bind _segmentlength (Variables|TrackSetup|GetSegmentLength))
  (bind _bankingmultiplier (Variables|OtherFunctionality|GetBankingMultiplier))
  (LocalVariables|SetLocal_CurrentLoopIndex LoopIndex)
  (LocalVariables|SetLocal_NextLoopIndex (+ LoopIndex 1))
  (LocalVariables|SetLocal_TrackElementMesh TrackElementMesh)
  (Utilities|FlowControl|Sequence
    (:then_0
      (if (or (.flipmesh (Utilities|Array|Get(acopy) (Variables|TrackSetup|GetRoadDataArray) (LocalVariables|GetLocal_CurrentLoopIndex))) (and (not (Utilities|IsValid (.overridemesh (Utilities|Array|Get(acopy) (Variables|TrackSetup|GetRoadDataArray) (LocalVariables|GetLocal_CurrentLoopIndex))))) (or (and (Variables|FirstandLastMeshSettings|GetFlipLastMesh) (== (+ (LocalVariables|GetLocal_CurrentLoopIndex) 1) (Variables|Default|GetPointsAmount))) (and (Variables|FirstandLastMeshSettings|GetFlipFirstMesh) (== (LocalVariables|GetLocal_CurrentLoopIndex) 0)))))
        (LocalVariables|SetLocal_StartLocation (Spline|GetLocationatDistanceAlongSpline (Variables|Default|GetTrackSpline) (* (LocalVariables|GetLocal_NextLoopIndex) (Variables|TrackSetup|GetSegmentLength)) "Local"))
        (LocalVariables|SetLocal_StartTangent (* (* (Spline|GetDirectionatDistanceAlongSpline (Variables|Default|GetTrackSpline) (* (LocalVariables|GetLocal_NextLoopIndex) (Variables|TrackSetup|GetSegmentLength)) "Local") (Variables|TrackSetup|GetSegmentLength)) -1))
        (LocalVariables|SetLocal_EndLocation (Spline|GetLocationatDistanceAlongSpline (Variables|Default|GetTrackSpline) (* (LocalVariables|GetLocal_CurrentLoopIndex) (Variables|TrackSetup|GetSegmentLength)) "Local"))
        (LocalVariables|SetLocal_EndTangent (* (* (Spline|GetDirectionatDistanceAlongSpline (Variables|Default|GetTrackSpline) (* (LocalVariables|GetLocal_CurrentLoopIndex) (Variables|TrackSetup|GetSegmentLength)) "Local") (Variables|TrackSetup|GetSegmentLength)) -1))
        (LocalVariables|SetLocal_StartRoll (+ (Math|Trig|DegreesToRadians (* -1 (+ (Variables|TrackSetup|GetBankingFix) 1.8e+02))) (* -1 (Math|Trig|DegreesToRadians (.trackbank (Utilities|Array|Get(acopy) (Variables|TrackSetup|GetRoadDataArray) (LocalVariables|GetLocal_NextLoopIndex)))))))
        (LocalVariables|SetLocal_StartScale (Math|Vector2D|MakeVector2D (* (.scalex (Utilities|Array|Get(acopy) (Variables|TrackSetup|GetRoadDataArray) (LocalVariables|GetLocal_NextLoopIndex))) (Variables|TrackSetup|GetGlobalScaleX)) (* (.scaley (Utilities|Array|Get(acopy) (Variables|TrackSetup|GetRoadDataArray) (LocalVariables|GetLocal_NextLoopIndex))) (Variables|TrackSetup|GetGlobalScaleY))))
        (LocalVariables|SetLocal_EndRoll (+ (Math|Trig|DegreesToRadians (* -1 (+ (Variables|TrackSetup|GetBankingFix) 1.8e+02))) (* -1 (Math|Trig|DegreesToRadians (.trackbank (Utilities|Array|Get(acopy) (Variables|TrackSetup|GetRoadDataArray) (LocalVariables|GetLocal_CurrentLoopIndex)))))))
        (LocalVariables|SetLocal_EndScale (Math|Vector2D|MakeVector2D (* (.scalex (Utilities|Array|Get(acopy) (Variables|TrackSetup|GetRoadDataArray) (LocalVariables|GetLocal_CurrentLoopIndex))) (Variables|TrackSetup|GetGlobalScaleX)) (* (.scaley (Utilities|Array|Get(acopy) (Variables|TrackSetup|GetRoadDataArray) (LocalVariables|GetLocal_CurrentLoopIndex))) (Variables|TrackSetup|GetGlobalScaleY))))
        (else
          (LocalVariables|SetLocal_StartLocation (Spline|GetLocationatDistanceAlongSpline (Variables|Default|GetTrackSpline) (* (LocalVariables|GetLocal_CurrentLoopIndex) (Variables|TrackSetup|GetSegmentLength)) "Local"))
          (LocalVariables|SetLocal_StartTangent (* (Spline|GetDirectionatDistanceAlongSpline (Variables|Default|GetTrackSpline) (* (LocalVariables|GetLocal_CurrentLoopIndex) (Variables|TrackSetup|GetSegmentLength)) "Local") (Variables|TrackSetup|GetSegmentLength)))
          (LocalVariables|SetLocal_EndLocation (Spline|GetLocationatDistanceAlongSpline (Variables|Default|GetTrackSpline) (* (LocalVariables|GetLocal_NextLoopIndex) (Variables|TrackSetup|GetSegmentLength)) "Local"))
          (LocalVariables|SetLocal_EndTangent (* (Spline|GetDirectionatDistanceAlongSpline (Variables|Default|GetTrackSpline) (* (LocalVariables|GetLocal_NextLoopIndex) (Variables|TrackSetup|GetSegmentLength)) "Local") (Variables|TrackSetup|GetSegmentLength)))
          (LocalVariables|SetLocal_StartRoll (+ (Math|Trig|DegreesToRadians (Variables|TrackSetup|GetBankingFix)) (Math|Trig|DegreesToRadians (.trackbank (Utilities|Array|Get(acopy) (Variables|TrackSetup|GetRoadDataArray) (LocalVariables|GetLocal_CurrentLoopIndex))))))
          (LocalVariables|SetLocal_StartScale (Math|Vector2D|MakeVector2D (* (.scalex (Utilities|Array|Get(acopy) (Variables|TrackSetup|GetRoadDataArray) (LocalVariables|GetLocal_CurrentLoopIndex))) (Variables|TrackSetup|GetGlobalScaleX)) (* (.scaley (Utilities|Array|Get(acopy) (Variables|TrackSetup|GetRoadDataArray) (LocalVariables|GetLocal_CurrentLoopIndex))) (Variables|TrackSetup|GetGlobalScaleY))))
          (LocalVariables|SetLocal_EndRoll (+ (Math|Trig|DegreesToRadians (Variables|TrackSetup|GetBankingFix)) (Math|Trig|DegreesToRadians (.trackbank (Utilities|Array|Get(acopy) (Variables|TrackSetup|GetRoadDataArray) (LocalVariables|GetLocal_NextLoopIndex))))))
          (LocalVariables|SetLocal_EndScale (Math|Vector2D|MakeVector2D (* (.scalex (Utilities|Array|Get(acopy) (Variables|TrackSetup|GetRoadDataArray) (LocalVariables|GetLocal_NextLoopIndex))) (Variables|TrackSetup|GetGlobalScaleX)) (* (.scaley (Utilities|Array|Get(acopy) (Variables|TrackSetup|GetRoadDataArray) (LocalVariables|GetLocal_NextLoopIndex))) (Variables|TrackSetup|GetGlobalScaleY))))))
      (LocalVariables|SetLocal_SegmentOrientation (.orientation (Utilities|Array|Get(acopy) (Variables|TrackSetup|GetRoadDataArray) (LocalVariables|GetLocal_CurrentLoopIndex)))))
    (:then_1
      (bind _returnvalue (AddComponent|AddSplineMeshComponent false))
      (Class|PrimitiveComponent|SetCullDistance _returnvalue (Variables|TrackSetup|GetRoadMeshDrawDistance))
      (SplineMesh|SetForwardAxis _returnvalue (LocalVariables|GetLocal_SegmentOrientation) true)
      (SplineMesh|SetSplineUpDir _returnvalue (Variables|TrackSetup|GetUpVectorFix) true)
      (Development|SetHiddeninGame _returnvalue HideInGame true)
      (LocalVariables|SetLocal_CurrentSplineMesh _returnvalue)
      (Components|StaticMesh|SetStaticMesh (LocalVariables|GetLocal_CurrentSplineMesh) (LocalVariables|GetLocal_TrackElementMesh))
      (SplineMesh|SetStartandEnd (LocalVariables|GetLocal_CurrentSplineMesh) (LocalVariables|GetLocal_StartLocation) (LocalVariables|GetLocal_StartTangent) (LocalVariables|GetLocal_EndLocation) (LocalVariables|GetLocal_EndTangent) true :!class /Script/Engine.SplineMeshComponent)
      (if (Variables|OtherFunctionality|GetPointBasedBanking)
        (if (Variables|TrackSetup|GetGizmoFix%20-IMPORTANT-)
          (Class|SplineMeshComponent|SetStartRoll (LocalVariables|GetLocal_CurrentSplineMesh) (/ (Class|SplineComponent|GetRollatDistanceAlongSpline _trackspline (* (LocalVariables|GetLocal_CurrentLoopIndex) _segmentlength) "Local") 6e+01) true)
          (Class|SplineMeshComponent|SetEndRoll (LocalVariables|GetLocal_CurrentSplineMesh) (/ (Class|SplineComponent|GetRollatDistanceAlongSpline _trackspline (* (+ (LocalVariables|GetLocal_CurrentLoopIndex) 1) _segmentlength) "Local") 6e+01) true)
          (else
            (Class|SplineMeshComponent|SetStartRoll (LocalVariables|GetLocal_CurrentSplineMesh) (+ (* (Class|SplineComponent|GetRollatDistanceAlongSpline _trackspline (* (LocalVariables|GetLocal_CurrentLoopIndex) _segmentlength) "Local") _bankingmultiplier) (Math|Trig|DegreesToRadians (Variables|TrackSetup|GetBankingFix))) true)
            (Class|SplineMeshComponent|SetEndRoll (LocalVariables|GetLocal_CurrentSplineMesh) (+ (* _bankingmultiplier (Class|SplineComponent|GetRollatDistanceAlongSpline _trackspline (* (+ (LocalVariables|GetLocal_CurrentLoopIndex) 1) _segmentlength) "Local")) (Math|Trig|DegreesToRadians (Variables|TrackSetup|GetBankingFix))) true)))
        (else
          (Class|SplineMeshComponent|SetStartRoll (LocalVariables|GetLocal_CurrentSplineMesh) (LocalVariables|GetLocal_StartRoll) true)
          (Class|SplineMeshComponent|SetEndRoll (LocalVariables|GetLocal_CurrentSplineMesh) (LocalVariables|GetLocal_EndRoll) true)))
      (SplineMesh|SetStartScale (LocalVariables|GetLocal_CurrentSplineMesh) (LocalVariables|GetLocal_StartScale) true :!class /Script/Engine.SplineMeshComponent)
      (SplineMesh|SetEndScale (LocalVariables|GetLocal_CurrentSplineMesh) (LocalVariables|GetLocal_EndScale) true :!class /Script/Engine.SplineMeshComponent)
      (Rendering|Material|SetMaterial (LocalVariables|GetLocal_CurrentSplineMesh) 0 (Variables|TrackSetup|GetMaterialOverride))
      (Collision|SetCollisionEnabled (LocalVariables|GetLocal_CurrentSplineMesh) (select EnableCollision "QueryAndPhysics" "NoCollision")))))

(fn GetNumPoints
  (params (Length :type Float%20%28single-precision%29))
  (bind _segmentlength (Variables|TrackSetup|GetSegmentLength))
  (bind _returnvalue (/ Length _segmentlength))
  (bind _returnvalue_2 (Math|Float|Truncate _returnvalue))
  (Math|Float|CompareFloat _segmentlength 1.0
    (:>
      (if (> (Math|Float|%(Float) Length _segmentlength) (* _segmentlength (Variables|TrackSetup|GetLastSegmentThreshold)))
        (return (+ _returnvalue_2 1))
        (else
          (return _returnvalue_2))))))

(fn ApplyOrientation
  (bind _roaddataarray (Variables|TrackSetup|GetRoadDataArray))
  (for (_array_element _array_index) _roaddataarray
    (if (not (.OverrideOrientation (Utilities|Struct|BreakRoadData _array_element)))
      (Utilities|Array|SetArrayElem _roaddataarray _array_index (Utilities|Struct|MakeRoadData (.TrackBank (Utilities|Struct|BreakRoadData _array_element)) (.ScaleX (Utilities|Struct|BreakRoadData _array_element)) (.ScaleY (Utilities|Struct|BreakRoadData _array_element)) (.OverrideMesh (Utilities|Struct|BreakRoadData _array_element)) (.CollisionOverride (Utilities|Struct|BreakRoadData _array_element)) (.AdditionalMeshOverride (Utilities|Struct|BreakRoadData _array_element)) (.FlipMesh (Utilities|Struct|BreakRoadData _array_element)) (Variables|TrackSetup|GetUniversalMeshOrientation) (.OverrideOrientation (Utilities|Struct|BreakRoadData _array_element)))))))